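; BP_Pistol is a pistol Blueprint that handles the visual feedback of firing.
; On FirePressed it spawns an auto-destroying Niagara muzzle flash attached to the muzzle, then plays a recoil timeline from the start.
; The timeline pitches MeshRoot and offsets it by ShootPistolOffset from the location cached at BeginPlay.
; It contains no projectile, trace or damage logic, and its camera shake nodes are disconnected.
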(event `self.ReceiveBeginPlay`
  (set `self.MeshRootLocation` (`SceneComponent.RelativeLocation` (`self.MeshRoot`))))

(event `self.BP_FirePressed`
  (bind _meshroot (`self.MeshRoot`))
  (`|ExecutionSequence`
    (:`then_0`
      (`NiagaraFunctionLibrary.SpawnSystemAttached` "/Game/Art/MuzzleFlash/NS_MuzzleFlash.NS_MuzzleFlash" (`self.MuzzleComponent`) "None" (0.0 0.0 0.0) (struct) "SnapToTarget" true))
    (:`then_1`
      (bind (_direction _progress) (`Timeline|Timeline` :!via `PlayFromStart`)
        (:`Update`
          (`SceneComponent.K2_SetRelativeRotation` _meshroot (`KismetMathLibrary.MakeRotator` 0.0 (* _progress -90.0)) false false)
          (`SceneComponent.K2_SetRelativeLocation` _meshroot (+ (* _progress (`self.ShootPistolOffset`)) (`self.MeshRootLocation`)) false false))))))

(fn `UserConstructionScript`)